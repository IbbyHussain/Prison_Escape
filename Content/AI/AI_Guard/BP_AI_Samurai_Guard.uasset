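; Samurai guard AI character that spawns with a weapon and weapon case, melee attacks with a slash montage, and can arrest the player.
; Tick watches the death flag to spawn a stamina pickup once, and point damage draws debug numbers at the hit location.
; Arresting sets game over, disables movement and loops an idle animation.
; Events toggle a face-player flag, but the smooth rotation logic that reads it is unconnected.
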(event `self.ReceiveBeginPlay`
  (`self.SpawnWeaponCase` "/Game/AI/AI_Guard/AI_Samurai_Weapon/BP_Samurai_WeaponCase.BP_Samurai_WeaponCase_C")
  (`self.SpawnWeapon` "/Game/AI/AI_Guard/AI_Samurai_Weapon/BP_AI_Samurai_Weapon.BP_AI_Samurai_Weapon_C"))

(event `self.ReceiveTick`
  (params (DeltaSeconds :type "Float (single-precision)"))
  (if (`self.bHasAIDied`)
    (`/Engine/EditorBlueprintResources/StandardMacros.DoOnce` false
      (:`Completed`
        (`GameplayStatics.GetAllActorsOfClass` null)
        (`self.SpawnStaminaPickup` "/Game/AI/AI_Guard/Misc/BP_StaminaPickup.BP_StaminaPickup_C")))))

(event `/Game/AI/AI_Guard/AI_Samurai_BehaviourTree/NewInterface.meleeAttack`
  (`|PlayMontage` (`self.Mesh`) "/Game/AI/AI_Guard/AI_Samurai_Animation/Sword_And_Shield_Slash_Montage.Sword_And_Shield_Slash_Montage"))

(event `EventFacePlayer`
  ;[1 1 1] smooth rotation in place
  (set `self.faceplayer` true))

(event `Event Stop Facing Player`
  ;[1 1 1] smooth rotation in place
  (set `self.faceplayer` false))

(event `self.ReceivePointDamage`
  (params (Damage :type "Float (single-precision)") (DamageType :type "DamageType Object Reference") (HitLocation :type "Vector Structure") (HitNormal :type "Vector Structure") (HitComponent :type "PrimitiveComponent Object Reference") (BoneName :type Name) (ShotFromDirection :type "Vector Structure") (InstigatedBy :type "Controller Object Reference") (DamageCauser :type "Actor Object Reference") (HitInfo :type "HitResult Structure (by ref)"))
  (`KismetSystemLibrary.DrawDebugString` HitLocation (`KismetStringLibrary.Conv_DoubleToString` Damage) null (struct :`R` 0.331357 :`G` 7.0 :`A` 1.0) 1.0))

(fn `AIArrestedPlayer`
  (set `self.IsGameOver` true)
  (set `CharacterMovementComponent.MaxWalkSpeed` 10.0 (`self.CharacterMovement`))
  (`MovementComponent.StopMovementImmediately` (`self.CharacterMovement`))
  (`CharacterMovementComponent.DisableMovement` (`self.CharacterMovement`))
  (`SkeletalMeshComponent.PlayAnimation` (`self.Mesh`) "/Game/AI/AI_Guard/AI_Samurai_Animation/Walk/Sword_And_Shield_Idle.Sword_And_Shield_Idle" true))

(fn `UserConstructionScript`)