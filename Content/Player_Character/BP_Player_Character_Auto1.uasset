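; Player character Blueprint that sets up the HUD, crosshair and socketed helmet, and handles arrest by freezing movement and input and showing a widget.
; E plays a camera shutter and reports a noise event.
; Tick stops sprinting while either anim Blueprint reports airborne, and each frame calls the first AK47 pickup's overlap handler and applies the armed anim class.
; Guard-distance and rifle-spawn logic is left unconnected.
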(event `self.ReceiveBeginPlay`
  (bind _returnvalue (`|CreateWidget` "/Game/UI/WBP_Player_HUD.WBP_Player_HUD_C"))
  (bind _returnvalue_2 (`|CreateWidget` "/Game/UI/WBP_CroosHair.WBP_CroosHair_C"))
  (`UserWidget.AddToViewport` _returnvalue 0)
  (`UserWidget.AddToViewport` _returnvalue_2 0)
  (bind _returnvalue_3 (`|SpawnActorFromClass` "/Game/Player_Character/BP_Helmet.BP_Helmet_C" (`SceneComponent.GetSocketTransform` (`self.Mesh`) "HelmetSocket" "RTS_World") "Undefined" "OverrideRootScale" null null))
  (`self.K2_AttachToComponent` _returnvalue_3 (`self.Mesh`) "HelmetSocket" "SnapToTarget" "SnapToTarget" "SnapToTarget" true))

(event `Key|E`
  (params (Key :type "Key Structure"))
  (bind _returnvalue (`self.K2_GetActorLocation`))
  ;[1 1 1] noise
  (:`Pressed`
    (`GameplayStatics.PlaySoundAtLocation` "/Engine/VREditor/Sounds/UI/Camera_Shutter.Camera_Shutter" _returnvalue (struct) 1.0 1.0 0.0 null null null)
    (`AISense_Hearing.ReportNoiseEvent` _returnvalue 1.0 self 0.0 "Noise")
    (`KismetSystemLibrary.PrintString` "Hello")))

(event `self.ReceiveTick`
  (params (DeltaSeconds :type "Float (single-precision)"))
  (bind _mesh (`self.Mesh`))
  (`|ExecutionSequence`
    (:`then_0`
      (bind _asabp_player (cast `/Game/Player_Character/Animations/UnArmed/ABP_Player` (`SkeletalMeshComponent.GetAnimInstance` (`self.Mesh`))))
      (if (`/Game/Player_Character/Animations/UnArmed/ABP_Player.IsInAir?` _asabp_player)
        (`KismetSystemLibrary.PrintString` "jumping" true true (struct :`G` 0.66 :`B` 1.0 :`A` 1.0) 0.0)
        (bind _asplayer_character (cast `Player_Character` (`GameplayStatics.GetPlayerCharacter` 0)))
        (`self.StopSprinting` _asplayer_character)))
    (:`then_1`
      (bind _asabp_player_armed (cast `/Game/Player_Character/Animations/Armed/ABP_Player_Armed` (`SkeletalMeshComponent.GetAnimInstance` (`self.Mesh`))))
      (if (`/Game/Player_Character/Animations/Armed/ABP_Player_Armed.ABP_IsInAir` _asabp_player_armed)
        (`KismetSystemLibrary.PrintString` "Armed jumping" true true (struct :`G` 0.66 :`B` 1.0 :`A` 1.0) 0.0)
        (bind _asplayer_character_2 (cast `Player_Character` (`GameplayStatics.GetPlayerCharacter` 0)))
        (`self.StopSprinting` _asplayer_character_2)))
    (:`then_3`
      (bind _outactors (`GameplayStatics.GetAllActorsOfClass` "/Game/Player_Character/Weapons/AK-47/AK47_Pickup/BP_AK47PickUp.BP_AK47PickUp_C"))
      (bind _asbp_ak47pick_up (cast `/Game/Player_Character/Weapons/AK-47/AK47_Pickup/BP_AK47PickUp` (`|GetArrayItem` _outactors)))
      (`C_AK47PickUp.OnOverlapBegin` :`self` _asbp_ak47pick_up :`OtherActor` self)
      (`SkeletalMeshComponent.SetAnimationMode` _mesh "AnimationBlueprint")
      (`SkeletalMeshComponent.K2_SetAnimInstanceClass` _mesh "/Game/Player_Character/Animations/Armed/ABP_Player_Armed.ABP_Player_Armed_C"))))

(event `Key|P`
  (params (Key :type "Key Structure"))
  ;[1 1 1] chnages abp blueprint
)

(fn `PlayerIsArrested`
  (`MovementComponent.StopMovementImmediately` (`self.CharacterMovement`))
  (`CharacterMovementComponent.DisableMovement` (`self.CharacterMovement`))
  (`self.DisableInput` (`GameplayStatics.GetPlayerController` 0))
  (bind _returnvalue (`|CreateWidget` "/Game/UI/Arrested/WBP_Arrested.WBP_Arrested_C"))
  (`UserWidget.AddToViewport` _returnvalue 0))

(fn `UserConstructionScript`)