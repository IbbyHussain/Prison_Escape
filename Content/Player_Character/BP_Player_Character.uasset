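; Player character Blueprint that adds the HUD, AI-audible noise and an arrested state.
; On BeginPlay it creates the Player_HUD widget, and on Tick it reads IsInAir from ABP_Player to stop sprinting while airborne, with debug prints.
; Pressing E plays a camera shutter sound and reports a "Noise"-tagged noise event at the player's location.
; PlayerIsArrested halts and disables movement, disables input and shows an arrested widget.
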(event `self.ReceiveBeginPlay`
  (`|ExecutionSequence`
    (:`then_0`
      (bind _returnvalue (`|CreateWidget` "/Game/UI/Player_HUD.Player_HUD_C"))
      (`UserWidget.AddToViewport` _returnvalue 0))))

(event `self.ReceiveTick`
  (params (DeltaSeconds :type "Float (single-precision)"))
  (bind _asabp_player (cast `/Game/Player_Character/Animations/ABP_Player` (`SkeletalMeshComponent.GetAnimInstance` (`self.Mesh`))))
  (if (`/Game/Player_Character/Animations/ABP_Player.IsInAir?` _asabp_player)
    (`KismetSystemLibrary.PrintString` "jumping" true true (struct :`G` 0.66 :`B` 1.0 :`A` 1.0) 0.0)
    (bind _asplayer_character (cast `Player_Character` (`GameplayStatics.GetPlayerCharacter` 0)))
    (`self.StopSprinting` _asplayer_character)
    (`KismetSystemLibrary.PrintString` "cnat sprint" true true (struct :`G` 0.66 :`B` 1.0 :`A` 1.0) 0.0)))

(event `Key|E`
  (params (Key :type "Key Structure"))
  (bind _returnvalue (`self.K2_GetActorLocation`))
  ;[1 1 1] noise
  (:`Pressed`
    (`GameplayStatics.PlaySoundAtLocation` "/Engine/VREditor/Sounds/UI/Camera_Shutter.Camera_Shutter" _returnvalue (struct) 1.0 1.0 0.0 null null null)
    (`AISense_Hearing.ReportNoiseEvent` _returnvalue 1.0 self 0.0 "Noise")
    (`KismetSystemLibrary.PrintString` "Hello")))

(fn `PlayerIsArrested`
  (`MovementComponent.StopMovementImmediately` (`self.CharacterMovement`))
  (`CharacterMovementComponent.DisableMovement` (`self.CharacterMovement`))
  (`self.DisableInput` (`GameplayStatics.GetPlayerController` 0))
  (bind _returnvalue (`|CreateWidget` "/Game/UI/Arrested/WBP_Arrested.WBP_Arrested_C"))
  (`UserWidget.AddToViewport` _returnvalue 0))

(fn `UserConstructionScript`)