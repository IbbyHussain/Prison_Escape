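; BP_CheckPoint is a trigger actor that saves or clears the player's checkpoint, depending on its CPLoad flag.
; On overlap with CPLoad set, it records player 0's location and writes it with Load true to the "Check" BP_SaveGame slot, creating the save if none exists.
; With CPLoad unset, it sets Load false in the existing save.
; The overlap does not filter which actor entered.
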(event `self.trigger.OnComponentBeginOverlap`
  (params (OverlappedComponent :type "PrimitiveComponent Object Reference") (OtherActor :type "Actor Object Reference") (OtherComp :type "PrimitiveComponent Object Reference") (OtherBodyIndex :type Integer) (bFromSweep :type Boolean) (SweepResult :type "HitResult Structure (by ref)"))
  (if (`self.CP_Load?`)
    (`|ExecutionSequence`
      (:`then_0`
        (bind _asbp_player_character (cast `/Game/Player_Character/BP_Player_Character_Auto1` (`GameplayStatics.GetPlayerCharacter` 0)))
        (set `self.CP_PlayerLocation` (`self.K2_GetActorLocation` _asbp_player_character))
        (`KismetSystemLibrary.PrintString` "check point reached"))
      (:`then_1`
        (bind _returnvalue (`GameplayStatics.DoesSaveGameExist` "Check"))
        (if _returnvalue
          (bind _returnvalue_2 (`GameplayStatics.LoadGameFromSlot` "Check"))
          (bind _asbp_save_game (cast `/Game/Player_Character/BP_SaveGame` _returnvalue_2))
          (set `/Game/Player_Character/BP_SaveGame.PlayerLocaion` (`self.CP_PlayerLocation`) _asbp_save_game)
          (set `/Game/Player_Character/BP_SaveGame.Load?` true _asbp_save_game)
          (`GameplayStatics.SaveGameToSlot` _asbp_save_game "Check")
          (else
            (bind _returnvalue_3 (`GameplayStatics.CreateSaveGameObject` "/Game/Player_Character/BP_SaveGame.BP_SaveGame_C"))
            (set `/Game/Player_Character/BP_SaveGame.PlayerLocaion` (`self.CP_PlayerLocation`) _returnvalue_3)
            (set `/Game/Player_Character/BP_SaveGame.Load?` true _returnvalue_3)
            (`GameplayStatics.SaveGameToSlot` _returnvalue_3 "Check")))))
    (else
      (bind _returnvalue_4 (`GameplayStatics.LoadGameFromSlot` "Check"))
      (bind _asbp_save_game_2 (cast `/Game/Player_Character/BP_SaveGame` _returnvalue_4))
      (set `/Game/Player_Character/BP_SaveGame.Load?` false _asbp_save_game_2)
      (`GameplayStatics.SaveGameToSlot` _asbp_save_game_2 "Check")
      (`KismetSystemLibrary.PrintString` "checkpoint cleared"))))

(fn `UserConstructionScript`)